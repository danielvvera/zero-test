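; Player Paper2D character (Zero) for a side-scrolling game, with walking, double jump, ground and air dash, and a three-slash combo.
; Input events set state flags that Tick reads to choose flipbooks and rotate the controller toward movement.
; Dashes drive velocity through Delay loops, Delays time the slashes, and landing resets air limits.
; BeginPlay starts a HUD and countdown ending in GameOver; GameComplete clears it and shows its own screen.
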(event `SonidoSalto`
  ;[1 1 1] Sonidos
  (if (not (`self.IsJumping`))
    (`GameplayStatics.PlaySound2D` "/Game/sonidos/Zero_sfx/voice/z_jump.z_jump" 1.0 1.0 0.0 null null)
    (`GameplayStatics.PlaySound2D` "/Game/sonidos/Zero_sfx/movement/zero_jump.zero_jump" 1.0 1.0 0.0 null null)))

(event `SonidoAtaque`
  (bind _slash2 (`self.Slash2`))
  (bind _slash1 (`self.Slash1`))
  (bind _returnvalue (not _slash2))
  (bind _returnvalue_2 (not (`self.Slash3`)))
  (bind _returnvalue_3 (and _returnvalue_2 _slash2))
  (bind _returnvalue_4 (and _slash1 _returnvalue))
  (bind _returnvalue_5 (or (`self.IsJumping`) (`NavMovementComponent.IsFalling` (`self.CharacterMovement`))))
  ;[1 1 1] Sonidos
  (if _returnvalue_3
    (`GameplayStatics.PlaySound2D` "/Game/sonidos/Zero_sfx/voice/zero_swing3.zero_swing3" 1.0 1.0 0.0 null null)
    (`GameplayStatics.PlaySound2D` "/Game/sonidos/Zero_sfx/saber/z_saber1.z_saber1" 1.0 1.0 0.0 null null :!label _label)
    (elif _returnvalue_4
      (`GameplayStatics.PlaySound2D` "/Game/sonidos/Zero_sfx/voice/zero_swing2.zero_swing2" 1.0 1.0 0.0 null null)
      (goto _label)
      (elif (or _returnvalue_5 (and (not _returnvalue_5) _returnvalue _returnvalue_2 (not _slash1)) _returnvalue_4 _returnvalue_3)
        (`GameplayStatics.PlaySound2D` "/Game/sonidos/Zero_sfx/voice/z_swing1.z_swing1" 1.0 1.0 0.0 null null)
        (goto _label)))))

(event `ActualizarAnimacion`
  (bind _returnvalue (`NavMovementComponent.IsFalling` (`self.CharacterMovement`)))
  ;[1 1 1] Animaciones
  (if (`self.IsJumping`)
    (`PaperFlipbookComponent.SetFlipbook` (`self.Sprite`) "/Game/texturas/ZeroX4/zero_jump.zero_jump")
    (set `self.ShortFall` true)
    (elif (and (`self.DashStop`) (not _returnvalue))
      (`PaperFlipbookComponent.SetFlipbook` (`self.Sprite`) "/Game/texturas/ZeroX4/zero_dashstop.zero_dashstop")
      (elif (and (`self.IsDashing`) (not (`self.IsJumping`)))
        (`PaperFlipbookComponent.SetFlipbook` (`self.Sprite`) "/Game/texturas/ZeroX4/zero_dash_full.zero_dash_full")
        (elif _returnvalue
          (`PaperFlipbookComponent.SetFlipbook` (`self.Sprite`) (select `bool` (`self.ShortFall`) :`false` "/Game/texturas/ZeroX4/zero_fall2.zero_fall2" :`true` "/Game/texturas/ZeroX4/zero_fall1.zero_fall1" :!type "PaperFlipbook Object Reference"))
          (else
            (`PaperFlipbookComponent.SetFlipbook` (`self.Sprite`) (select `bool` (> (`KismetMathLibrary.VSize` (`MovementComponent.Velocity` (`self.CharacterMovement`))) 0.0) :`false` "/Game/texturas/ZeroX4/zero_idle.zero_idle" :`true` "/Game/texturas/ZeroX4/zero_walk.zero_walk" :!type "PaperFlipbook Object Reference"))))))))

(event `ActualizarRotacion`
  ;[1 1 1] Rotación paper character
  (`/Engine/EditorBlueprintResources/StandardMacros.CompareFloat` (.x (`MovementComponent.Velocity` (`self.CharacterMovement`)))
    (:`>`
      (`Controller.SetControlRotation` (`self.GetController`) (`KismetMathLibrary.MakeRotator` 0.0)))
    (:`<`
      (`Controller.SetControlRotation` (`self.GetController`) (`KismetMathLibrary.MakeRotator` 0.0 0.0 180.0)))))

(event `SonidoDash`
  ;[1 1 1] Sonidos
  (if (and (`self.IsDashing`) (< (`self.AirDashCuantity`) (`self.MaxAirDashCuantity`)) (`self.CanAirDash`) (> (`self.max_jumps`) (`self.jump_counter`)))
    (`GameplayStatics.PlaySound2D` "/Game/sonidos/Zero_sfx/movement/zero_dash_start.zero_dash_start" 1.0 1.0 0.0 null null)))

(event `SonidoDashStop`
  ;[1 1 1] Sonidos
  (if (and (not (`NavMovementComponent.IsFalling` (`self.CharacterMovement`))) (`self.DashStop`))
    (`GameplayStatics.PlaySound2D` "/Game/sonidos/Zero_sfx/movement/zero_dash_stop.zero_dash_stop" 1.0 1.0 0.0 null null)))

(event `Fall`
  ;[1 1 1] Caída
  (if (`NavMovementComponent.IsFalling` (`self.CharacterMovement`))
    (`KismetSystemLibrary.Delay` 2.0)
    (set `self.ShortFall` false)
    (else
      (set `self.ShortFall` true))))

(event `InputAction|dash`
  (params (Key :type "Key Structure"))
  (bind _returnvalue_x (`KismetMathLibrary.BreakVector` (`self.GetActorForwardVector`)))
  (bind (_returnvalue_x_2 _returnvalue_y _returnvalue_z) (`KismetMathLibrary.BreakVector` (`self.GetActorForwardVector`)))
  (bind _returnvalue_x_3 (`KismetMathLibrary.BreakVector` (`self.GetActorForwardVector`)))
  (bind _charactermovement (`self.CharacterMovement`))
  (bind _dashcount (`self.DashCount`))
  (bind _airdashcount (`self.AirDashCount`))
  (bind _charactermovement_2 (`self.CharacterMovement`))
  ;[1 1 1] Dash
  (:`Pressed`
    (set `self.Slash1` false)
    (set `self.Slash2` false)
    (set `self.Slash3` false)
    (set `self.IsDashing` true)
    (set `CharacterMovementComponent.GroundFriction` 0.0 _charactermovement_2)
    (`self.SonidoDash`)
    (if (`NavMovementComponent.IsFalling` _charactermovement_2)
      ;[1 1 1] AirDash
      (`self.StopJumping`)
      (set `self.IsJumping` false)
      (if (and (`self.CanAirDash`) (> (`self.max_jumps`) (`self.jump_counter`)))
        (if (< (`self.AirDashCuantity`) (`self.MaxAirDashCuantity`))
          (set `self.AirDashCuantity` (+ (`self.AirDashCuantity`) 1))
          (if (`self.IsDashing`) :!label _label_2
            (set `MovementComponent.Velocity` (`KismetMathLibrary.MakeVector` (* _returnvalue_x_3 (`self.DashVelocity`)) 0.0 91.0) (`self.CharacterMovement`))
            (`KismetSystemLibrary.Delay` 0.05)
            (set `self.AirDashCount` (+ _airdashcount 1))
            (if (>= _airdashcount (`self.AirDashLength`))
              (set `self.IsDashing` false)
              (set `self.AirDashCount` 0)
              (set `CharacterMovementComponent.GroundFriction` 30.0 (`self.CharacterMovement`))
              (set `self.CanAirDash` false)
              (else
                (goto _label_2)))
            (else
              (set `self.AirDashCount` 0)
              (set `CharacterMovementComponent.GroundFriction` 30.0 (`self.CharacterMovement`))
              (set `self.CanAirDash` false)))
          (`MovementComponent.StopMovementImmediately` (`self.CharacterMovement`)))
        (else
          (set `self.IsDashing` false)))
      (else
        ;[1 1 1] GroundDash
        (if (`self.IsDashing`) :!label _label_3
          (set `MovementComponent.Velocity` (`KismetMathLibrary.MakeVector` (* _returnvalue_x (`self.DashVelocity`))) (`self.CharacterMovement`))
          (`KismetSystemLibrary.Delay` 0.05)
          (set `self.DashCount` (+ _dashcount 1))
          (if (>= _dashcount (`self.DashLength`))
            (set `CharacterMovementComponent.GroundFriction` 30.0 (`self.CharacterMovement`))
            (set `self.IsDashing` false)
            (set `self.DashCount` 0)
            (set `MovementComponent.Velocity` (0.0 0.0 0.0) (`self.CharacterMovement`))
            (set `self.DashStop` true)
            (`self.SonidoDashStop`)
            (`KismetSystemLibrary.Delay` 0.2)
            (set `self.DashStop` false)
            (elif (`NavMovementComponent.IsFalling` (`self.CharacterMovement`))
              (if (not (or (`PlayerController.IsInputKeyDown` (`GameplayStatics.GetPlayerController` 0) "A") (`PlayerController.IsInputKeyDown` (`GameplayStatics.GetPlayerController` 0) "D")))
                (set `MovementComponent.Velocity` (`KismetMathLibrary.MakeVector` 0.0 0.0 _returnvalue_z) (`self.CharacterMovement`)))
              (set `CharacterMovementComponent.GroundFriction` 30.0 _charactermovement)
              (set `CharacterMovementComponent.MaxWalkSpeed` 800.0 _charactermovement)
              (set `self.IsDashing` false)
              (set `self.DashCount` 0)
              (set `self.CanAirDash` false)
              (else
                (goto _label_3))))
          (else
            (set `CharacterMovementComponent.GroundFriction` 30.0 (`self.CharacterMovement`))
            (set `self.DashCount` 0)
            (set `self.DashStop` true)
            (`self.SonidoDashStop`)
            (`KismetSystemLibrary.Delay` 0.2)
            (set `self.DashStop` false)
            (set `self.IsDashing` false))))))
  (:`Released`
    (set `self.IsDashing` false)
    (set `CharacterMovementComponent.GroundFriction` 30.0 _charactermovement_2)))

(event `InputAction|salto`
  (params (Key :type "Key Structure"))
  (bind _jump_counter (`self.jump_counter`))
  ;[1 1 1] Salto
  (:`Pressed`
    (if (and (> (`self.max_jumps`) _jump_counter) (< (`self.AirDashCuantity`) (`self.MaxAirDashCuantity`)) (`self.CanAirDash`))
      (set `self.jump_counter` (+ _jump_counter 1))
      (`self.Jump`)
      (`self.SonidoSalto`)
      (set `self.IsJumping` true)
      (`KismetSystemLibrary.Delay` 0.5))
    (set `self.IsJumping` false :!label _label_4))
  (:`Released`
    (`self.StopJumping`)
    (goto _label_4)))

(event `self.OnLanded`
  (params (Hit :type "HitResult Structure (by ref)"))
  ;[1 1 1] Aterrizar
  (set `self.jump_counter` 0)
  (set `self.Slash1` false)
  (set `self.IsJumping` false)
  (set `self.IsDashing` false)
  (set `self.AirDashCuantity` 0)
  (set `self.CanAirDash` true)
  (set `self.ShortFall` true)
  (set `CharacterMovementComponent.MaxWalkSpeed` 600.0 (`self.CharacterMovement`))
  (`GameplayStatics.PlaySound2D` "/Game/sonidos/Zero_sfx/movement/zero_land.zero_land" 1.0 1.0 0.0 null null))

(event `InputAxis|MoverDerechaIzquierda`
  (params (AxisValue :type "Float (single-precision)"))
  ;[1 1 1] Caminar
  (if (`self.CanMove`)
    (`self.AddMovementInput` (0.6 0.0 0.0) AxisValue)
    (else
      (`MovementComponent.StopMovementImmediately` (`self.CharacterMovement`)))))

(event `InputAction|ataque`
  (params (Key :type "Key Structure"))
  (bind _returnvalue (or (`self.IsJumping`) (`NavMovementComponent.IsFalling` (`self.CharacterMovement`))))
  (bind _returnvalue_2 (not _returnvalue))
  ;[1 1 1] Ataque
  (:`Pressed`
    (set `self.IsDashing` false)
    (if (and (not (`self.Slash1`)) (`self.Slash2`) _returnvalue_2)
      (`self.SonidoAtaque`)
      (set `self.Slash3` true)
      (set `self.CanMove` false)
      (`KismetSystemLibrary.Delay` 0.5)
      (set `self.Slash3` false)
      (set `self.Slash1` false :!label _label_5)
      (set `self.CanMove` true)
      (elif (and (`self.Slash1`) (not (`self.Slash2`)) (not (`self.Slash3`)) _returnvalue_2)
        (`self.SonidoAtaque`)
        (set `self.Slash2` true)
        (set `self.CanMove` false)
        (`KismetSystemLibrary.Delay` 0.3)
        (set `self.Slash2` false)
        (goto _label_5)
        (elif (not (`self.Slash1`))
          (`self.SonidoAtaque`)
          (set `self.Slash1` true)
          (if (not _returnvalue)
            (set `self.CanMove` false))
          (`KismetSystemLibrary.Delay` 0.2)
          (goto _label_5))))))

(event `self.ReceiveTick`
  (params (DeltaSeconds :type "Float (single-precision)"))
  ;[1 1 1] Event Tick
  (`self.Fall`)
  (if (`self.Slash3`)
    (`self.Ataque_3`)
    (`self.ActualizarRotacion` :!label _label_6)
    (elif (`self.Slash2`)
      (`self.Ataque_2`)
      (goto _label_6)
      (elif (`self.Slash1`)
        (`self.ataque_1`)
        (if (or (`NavMovementComponent.IsFalling` (`self.CharacterMovement`)) (`self.IsJumping`))
          (goto _label_6))
        (else
          (`self.ActualizarAnimacion`)
          (goto _label_6))))))

(event `Ataque_1`
  ;[1 1 1] Ataque
  (`PaperFlipbookComponent.SetFlipbook` (`self.Sprite`) (select `bool` (or (`self.IsJumping`) (`NavMovementComponent.IsFalling` (`self.CharacterMovement`))) :`false` "/Game/texturas/ZeroX4/zero_slash1.zero_slash1" :`true` "/Game/texturas/ZeroX4/zero_slash0.zero_slash0" :!type "PaperFlipbook Object Reference")))

(event `Ataque_2`
  ;[1 1 1] Ataque
  (`PaperFlipbookComponent.SetFlipbook` (`self.Sprite`) "/Game/texturas/ZeroX4/zero_slash2.zero_slash2"))

(event `Ataque_3`
  ;[1 1 1] Ataque
  (`PaperFlipbookComponent.SetFlipbook` (`self.Sprite`) "/Game/texturas/ZeroX4/zero_slash3.zero_slash3"))

(event `self.ReceiveBeginPlay`
  ;[1 1 1] Timer
  (bind _returnvalue (`|CreateWidget` "/Game/widgets/HUDTimer.HUDTimer_C"))
  (`UserWidget.AddToViewport` _returnvalue 0)
  (bind _returnvalue_2 (`KismetSystemLibrary.K2_SetTimerDelegate` (delegate `FinTiempo`) (`self.TiempoJuego`)))
  (set `self.Timer` _returnvalue_2))

(event `FinTiempo`
  ;[1 1 1] Timer
  (`self.GameOver`))

(fn `GameComplete`
  (bind _returnvalue (`GameplayStatics.GetPlayerController` 0))
  (`self.DisableInput` null)
  (bind _returnvalue_2 (`|CreateWidget` "/Game/widgets/HUDGameComplete.HUDGameComplete_C" _returnvalue))
  (`UserWidget.AddToViewport` _returnvalue_2 0)
  (`KismetSystemLibrary.K2_ClearAndInvalidateTimerHandle` (`self.Timer`))
  (`WidgetBlueprintLibrary.SetInputMode_UIOnlyEx` _returnvalue _returnvalue_2 "LockAlways")
  (set `PlayerController.bShowMouseCursor` true _returnvalue))

(fn `GameOver`
  (bind _returnvalue (`GameplayStatics.GetPlayerController` 0))
  (`self.DisableInput` null)
  (bind _returnvalue_2 (`|CreateWidget` "/Game/widgets/HUDGameOver.HUDGameOver_C" _returnvalue))
  (`UserWidget.AddToViewport` _returnvalue_2 0)
  (`WidgetBlueprintLibrary.SetInputMode_UIOnlyEx` _returnvalue _returnvalue_2 "LockAlways")
  (set `PlayerController.bShowMouseCursor` true _returnvalue))

(fn `UserConstructionScript`
  (bind _charactermovement (`self.CharacterMovement`))
  (set `self.max_jumps` 2)
  (set `self.JumpMaxHoldTime` 0.5)
  (set `CharacterMovementComponent.GravityScale` 3.0 _charactermovement)
  (set `CharacterMovementComponent.GroundFriction` 30.0 _charactermovement)
  (set `CharacterMovementComponent.JumpZVelocity` 400.0 _charactermovement)
  (set `CharacterMovementComponent.AirControl` 1.0 _charactermovement)
  (set `CharacterMovementComponent.AirControlBoostMultiplier` 0.0 _charactermovement)
  (set `CharacterMovementComponent.AirControlBoostVelocityThreshold` 0.0 _charactermovement)
  (set `CharacterMovementComponent.MaxAcceleration` 7000.0 _charactermovement)
  (set `PhysicsVolume.TerminalVelocity` 800.0 (`MovementComponent.GetPhysicsVolume` _charactermovement)))